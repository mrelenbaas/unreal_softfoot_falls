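; Timer_Blueprint is an actor that measures frame rate and shows it on a TextRender component in the world.
; Tick accumulates delta time and counts frames.
; Once the elapsed time exceeds PERIOD, it stores the count as Fps, writes it to the text as an integer and resets both accumulators.
; The value is the raw frame count per period, not divided by the elapsed time.
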(event EventBeginPlay)

(event EventTick
  (params (DeltaSeconds :type Float%20%28single-precision%29))
  (Variables|Default|Setcurrent (+ DeltaSeconds (Variables|Default|Getcurrent)))
  (Variables|Default|Setcount (+ (Variables|Default|Getcount) 1))
  (if (> (Variables|Default|Getcurrent) (Variables|Default|GetPERIOD))
    (Variables|Default|Setfps (Variables|Default|Getcount))
    (Variables|Default|Setcount 0)
    (Variables|Default|Setcurrent 0.0)
    (Rendering|Components|TextRender|SetText (Variables|Default|GetTextRender) (Utilities|Text|ToText(Integer) (Variables|Default|Getfps)))))

(fn ConstructionScript)